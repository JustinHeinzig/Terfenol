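; S-D-F world Blueprint whose cube material reflects how far its Density, Specularity and Temperature are from the values held by a UMG widget.
; Each Tick passes the three absolute differences through exponential decay math expressions (A·e^(-K·T)).
; One minus each result drives the matching scalar parameter, so it is zero on a match and approaches one as the gap grows.
; BeginPlay creates the dynamic material instance and sets those parameters.
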(event EventBeginPlay
  (bind _returnvalue (Math|Float|MakeLiteralFloat 1.0))
  (bind _returnvalue_2 (Rendering|Material|CreateDynamicMaterialInstance (Variables|Default|GetCube) 0 "/Game/Materials/S-D-F-DynamicMaterial.S-D-F-DynamicMaterial" "None" :!class /Script/Engine.PrimitiveComponent))
  (Rendering|Material|SetScalarParameterValue _returnvalue_2 "Density" (- _returnvalue (stale EventTick _output_get)) :!class /Script/Engine.MaterialInstanceDynamic)
  (Rendering|Material|SetScalarParameterValue _returnvalue_2 "Temperature" (- _returnvalue (stale EventTick _output_get_3)) :!class /Script/Engine.MaterialInstanceDynamic)
  (Rendering|Material|SetScalarParameterValue _returnvalue_2 "Specularity" (- _returnvalue (stale EventTick _output_get_2)) :!class /Script/Engine.MaterialInstanceDynamic))

(event EventTick
  (params (DeltaSeconds :type Float%20%28single-precision%29))
  (bind _returnvalue (Math|Float|MakeLiteralFloat 1.0))
  (bind _umgwidgetref (Variables|Default|GetUMGWidgetRef))
  (bind _output_get (Variables|Default|SetAbsDensDif (|(a*(e((((0-1)*k)*t)))) 1.0 0.25 (Math|Float|Absolute(Float) (- (Variables|Default|GetDensity) (Variables|/Game/Tablet/UI/TabletUI.TabletUI_C|GetDensityValue _umgwidgetref))))))
  (bind _output_get_2 (Variables|Default|SetAbsSpecularityDif (|(a*(e((((0-1)*k)*t)))) 1.0 0.25 (Math|Float|Absolute(Float) (- (Variables|Default|GetSpecularity) (Variables|/Game/Tablet/UI/TabletUI.TabletUI_C|GetSpecularityValue _umgwidgetref))))))
  (bind _output_get_3 (Variables|Default|SetAbsTemperatureDif (|(a*(e((((0-1)*k)*t)))) 1.0 0.25 (Math|Float|Absolute(Float) (- (Variables|Default|GetTemperature) (Variables|/Game/Tablet/UI/TabletUI.TabletUI_C|GetTemperatureValue _umgwidgetref))))))
  (Rendering|Material|SetScalarParameterValue (stale EventBeginPlay _returnvalue_2) "Density" (- _returnvalue _output_get) :!class /Script/Engine.MaterialInstanceDynamic)
  (Rendering|Material|SetScalarParameterValue (stale EventBeginPlay _returnvalue_2) "Temperature" (- _returnvalue _output_get_3) :!class /Script/Engine.MaterialInstanceDynamic)
  (Rendering|Material|SetScalarParameterValue (stale EventBeginPlay _returnvalue_2) "Specularity" (- _returnvalue _output_get_2) :!class /Script/Engine.MaterialInstanceDynamic))

(fn ConstructionScript)